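; Brick spawner actor for Breakout that places child actor components and spawns bricks from BrickList.
; The construction script sizes the box, collects eight arrow transforms and adds nine child actor components at random picks, so positions can repeat.
; BeginPlay appends BrickList's first entry, then loops from the new index to 10, spawning that first class at the box's location and printing each index.
; The node setting the child actor class is disconnected.
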(event EventBeginPlay
  (bind _bricklist (Variables|Default|GetBrickList))
  (bind _output (Utilities|Array|Get(acopy) _bricklist))
  (bind _returnvalue (Utilities|Array|Add _bricklist _output))
  (for _index (range _returnvalue 10)
    (Game|SpawnActorfromClass _output (Math|Transform|MakeTransform (Transformation|GetWorldLocation (Variables|Default|GetBox)) "0.000000, 0,90.000000" "1,1,1") "Undefined" 0 0)
    (Development|PrintString (Utilities|String|ToString(Integer) _index))))

(fn ConstructionScript
  (Components|Box|SetBoxExtent (Variables|Default|GetBox) (Variables|Default|GetInBoxExtent) true)
  (CallFunction|SetSpawnPoint)
  (CallFunction|ItemSpawn))

(fn SetSpawnPoint
  (Variables|Default|SetSpawnPoints (Utilities|Array|MakeArray (Transformation|GetRelativeTransform (Variables|Default|GetArrow1)) (Transformation|GetRelativeTransform (Variables|Default|Get%20Arrow2)) (Transformation|GetRelativeTransform (Variables|Default|Get%20Arrow3)) (Transformation|GetRelativeTransform (Variables|Default|Get%20Arrow4)) (Transformation|GetRelativeTransform (Variables|Default|Get%20Arrow5)) (Transformation|GetRelativeTransform (Variables|Default|Get%20Arrow6)) (Transformation|GetRelativeTransform (Variables|Default|Get%20Arrow7)) (Transformation|GetRelativeTransform (Variables|Default|Get%20Arrow8)))))

(fn ItemSpawn
  (bind _spawnpoints (Variables|Default|GetSpawnPoints))
  (bind _returnvalue (Utilities|Array|LastIndex _spawnpoints))
  (bind _returnvalue_2 (Math|Random|RandomIntegerinRange 0 _returnvalue))
  (bind _output (Utilities|Array|Get(acopy) _spawnpoints _returnvalue_2))
  (bind _returnvalue_3 (AddComponent|AddChildActorComponent false _output))
  (AddComponent|AddChildActorComponent false _output)
  (AddComponent|AddChildActorComponent false _output)
  (AddComponent|AddChildActorComponent false _output)
  (AddComponent|AddChildActorComponent false _output)
  (AddComponent|AddChildActorComponent false _output)
  (AddComponent|AddChildActorComponent false _output)
  (AddComponent|AddChildActorComponent false _output)
  (AddComponent|AddChildActorComponent false _output))