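; Breakout ball actor that rides the player paddle's arrow until Lancer activates it and launches it with a velocity-change impulse.
; Every tick, ClampVelocity forces the physics velocity to the Vitesse speed and snaps it to horizontal diagonals, rotating by 45°, rounding yaw to 90° steps, then rotating back.
; When destroyed, it reports the lost ball to the game mode and has the paddle spawn a replacement.
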(event Custom|Lancer
  (params (Direction :type Vector))
  ;[1 1 1] Lancer la ball
  (Variables|Default|SetActive true)
  (Physics|AddImpulse (Variables|Default|GetBall) Direction "None" true))

(event Custom|MajPosition
  ;[1 1 1] Mise à jour de la position de la ball
  (if (not (Variables|Default|GetActive))
    (Transformation|SetActorLocation (Transformation|GetWorldLocation (Variables|/Game/Breakout/Core/Actors/BP_PaddlePlayer.BP_PaddlePlayer_C|GetArrow (Variables|Default|GetPaddle_Joueur))) false false)))

(event Custom|ClampVelocity
  (bind _returnvalue (Transformation|GetVelocity))
  (bind _returnvalue_2 (Math|Rotator|MakeRotator 0.0 0.0 45.0))
  (bind _vitesse (Variables|Default|GetVitesse))
  (bind _returnvalue_3 (Math|Vector|ClampVectorSize _returnvalue _vitesse _vitesse))
  ;[1 1 1] Clamp ball velocity
  (Physics|SetPhysicsLinearVelocity (Variables|Default|GetBall) (* (Math|Vector|UnrotateVector (Math|Rotator|GetRotationXVector (Math|Rotator|MakeRotator 0.0 0.0 (|((round((A/B)))*B) (.yaw (Math|Rotator|MakeRotfromX (Math|Vector|RotateVector _returnvalue_3 _returnvalue_2))) 9e+01))) _returnvalue_2) (Math|Vector|VectorLength _returnvalue_3)) false "None"))

(event EventBeginPlay
  ;[1 1 1] Obtenir le paddle joueur
  (bind _asbp_paddle_player (Utilities|Casting|CastToBP_PaddlePlayer (Pawn|GetControlledPawn (Game|GetPlayerController 0))))
  (Variables|Default|SetPaddle_Joueur _asbp_paddle_player)
  ;[1 1 1] Obtenir le mode de jeu du  break out
  (bind _asbp_game_mode (Utilities|Casting|CastToBP_GameMode (Game|GetGameMode)))
  (Variables|Default|SetGameMode _asbp_game_mode))

(event EventTick
  (params (DeltaSeconds :type Float%20%28single-precision%29))
  (CallFunction|MajPosition)
  (CallFunction|ClampVelocity))

(event EventDestroyed
  ;[1 1 1] Spawn une nouvelle ball apres avoir été detruite
  (Default|BallPerdu (Variables|Default|GetGameMode))
  (Default|SpawnNouvelleBall (Variables|Default|GetPaddle_Joueur)))

(fn ConstructionScript
  (|CallParentFunction))