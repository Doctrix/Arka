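; Breakout brick that takes up to three ball hits, depending on its starting collision flags, before it is destroyed.
; The construction script derives color and point value from those flags.
; Each BP_Ball end overlap recolors it yellow, then red, through new dynamic materials, then destroys it.
; On destruction it sends its index to the BreakoutLevel01 level script, plays explosion effects and adds score via the game mode; bonus-spawning code is disconnected.
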(event EventDestroyed
  (Class|BPILevel|SetIndexBlocks(Message) (Class|GameplayStatics|GetStreamingLevel "BreakoutLevel01") (Variables|Default|GetIndex))
  (Audio|PlaySound2D "/Game/StarterContent/Audio/Explosion_Cue.Explosion_Cue" 1.0 1.0 0.0 0 0)
  (bind _block (Variables|Default|GetBlock)
    (:then
      (Effects|SpawnEmitteratLocation "/Game/StarterContent/Particles/P_Explosion.P_Explosion" (Transformation|GetWorldLocation _block) "0, 0, 0" "1.000000,1.000000,1.000000" true "AutoRelease")
      (bind _asbp_game_mode_breakout (Utilities|Casting|CastToBP_GameModeBreakout (Game|GetGameMode)))
      (Default|UpdateScore _asbp_game_mode_breakout (Variables|Default|GetPoints)))
    (:else)))

(event Collision|EventActorEndOverlap
  (params (OtherActor :type Actor%20Object%20Reference))
  (Utilities|Casting|CastToBP_Ball OtherActor)
  (if (Variables|Default|Get1Colission)
    (Actor|DestroyActor self)
    (elif (Variables|Default|Get2Colission)
      (bind _returnvalue (Rendering|Material|CreateDynamicMaterialInstance (Variables|Default|GetBlock) 0 "/Game/Breakout/MaterialLibrary/Materials/M_Base.M_Base" "None" :!class /Script/Engine.PrimitiveComponent))
      (Rendering|Material|SetVectorParameterValue _returnvalue "Couleur" "(R=1.000000,G=0.000000,B=0.000000,A=0.000000)" :!class /Script/Engine.MaterialInstanceDynamic)
      (Variables|Default|Set1Colission true)
      (else
        (bind _returnvalue_2 (Rendering|Material|CreateDynamicMaterialInstance (Variables|Default|GetBlock) 0 "/Game/Breakout/MaterialLibrary/Materials/M_Base.M_Base" "None" :!class /Script/Engine.PrimitiveComponent))
        (Rendering|Material|SetVectorParameterValue _returnvalue_2 "Couleur" "(R=1.000000,G=1.000000,B=0.000000,A=0.000000)" :!class /Script/Engine.MaterialInstanceDynamic)
        (Variables|Default|Set2Colission true)))))

(fn ConstructionScript
  (bind _block (Variables|Default|GetBlock))
  (if (Variables|Default|Get1Colission)
    (bind _returnvalue (Rendering|Material|CreateDynamicMaterialInstance _block 0 "/Game/Breakout/MaterialLibrary/Materials/M_Base.M_Base" "None" :!class /Script/Engine.PrimitiveComponent))
    (Rendering|Material|SetVectorParameterValue _returnvalue "Couleur" "(R=1.000000,G=0.000000,B=0.000000,A=0.000000)" :!class /Script/Engine.MaterialInstanceDynamic)
    (Variables|Default|SetPoints 5)
    (elif (Variables|Default|Get2Colission)
      (bind _returnvalue_2 (Rendering|Material|CreateDynamicMaterialInstance _block 0 "/Game/Breakout/MaterialLibrary/Materials/M_Base.M_Base" "None" :!class /Script/Engine.PrimitiveComponent))
      (Rendering|Material|SetVectorParameterValue _returnvalue_2 "Couleur" "(R=1.000000,G=1.000000,B=0.000000,A=0.000000)" :!class /Script/Engine.MaterialInstanceDynamic)
      (Variables|Default|SetPoints 15)
      (else
        (bind _returnvalue_3 (Rendering|Material|CreateDynamicMaterialInstance _block 0 "/Game/Breakout/MaterialLibrary/Materials/M_Base.M_Base" "None" :!class /Script/Engine.PrimitiveComponent))
        (Rendering|Material|SetVectorParameterValue _returnvalue_3 "Couleur" (Variables|Default|GetColorBlock) :!class /Script/Engine.MaterialInstanceDynamic)
        (Variables|Default|SetPoints 30)))))