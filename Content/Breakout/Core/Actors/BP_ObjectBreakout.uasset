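; BP_ObjectBreakout is a pickup actor in the Breakout game that the player paddle collects on contact.
; Its construction script uses the Type enum to give the mesh a gold, poison or blue material through a dynamic material instance.
; When BP_PaddlePlayer overlaps the Sphere, it calls BonusCollectPlayer on the paddle's GameMode with a fixed argument, regardless of Type, then destroys itself.
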(event OnComponentBeginOverlap(Sphere)
  (params (OverlappedComponent :type Primitive%20Component%20Object%20Reference) (OtherActor :type Actor%20Object%20Reference) (OtherComp :type Primitive%20Component%20Object%20Reference) (OtherBodyIndex :type Integer) (bFromSweep :type Boolean) (SweepResult :type Hit%20Result%20Structure%20%28by%20ref%29))
  (bind _asbp_paddle_player (Utilities|Casting|CastToBP_PaddlePlayer OtherActor))
  (Default|BonusCollectPlayer (Variables|/Game/Breakout/Core/Actors/BP_PaddlePlayer.BP_PaddlePlayer_C|GetGameMode _asbp_paddle_player) 1)
  (Actor|DestroyActor))

(fn ConstructionScript
  (if (Utilities|Enum|Equal(Enum) (Variables|Default|Gettype) "NewEnumerator1")
    (Rendering|Material|CreateDynamicMaterialInstance (Variables|Default|GetMesh) 0 "/Game/Breakout/MaterialLibrary/Materials/Instances/MI_Or.MI_Or" "None" :!class /Script/Engine.PrimitiveComponent)
    (elif (Utilities|Enum|Equal(Enum) (Variables|Default|Gettype) "NewEnumerator3")
      (Rendering|Material|CreateDynamicMaterialInstance (Variables|Default|GetMesh) 0 "/Game/Breakout/MaterialLibrary/Materials/Instances/MI_Poison.MI_Poison" "None" :!class /Script/Engine.PrimitiveComponent)
      (elif (Utilities|Enum|Equal(Enum) (Variables|Default|Gettype) "NewEnumerator2")
        (Rendering|Material|CreateDynamicMaterialInstance (Variables|Default|GetMesh) 0 "/Game/Breakout/MaterialLibrary/Materials/Instances/Metal/MI_Bleu.MI_Bleu" "None" :!class /Script/Engine.PrimitiveComponent)))))