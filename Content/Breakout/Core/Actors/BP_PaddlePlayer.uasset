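; Player paddle for the Breakout game, which moves on input and launches the ball.
; Movement applies impulses to the paddle mesh while the game state allows, with vertical movement behind an optional flag.
; Game mode events trigger a position reset to the saved start location and spawn a new ball at the arrow, also done on BeginPlay.
; Shoot launches an inactive ball along the arrow's forward direction.
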(event Custom|SpawnNewBall
  ;[1 1 1] Faire apparaitre une nouvelle balle
  (if (Utilities|Enum|Equal(Enum) (Variables|/Game/Breakout/Core/Engine/BP_GameModeBreakout.BP_GameModeBreakout_C|GetStatsGame (Variables|Default|GetGameMode)) "NewEnumerator0")
    (bind _returnvalue (Game|SpawnActorfromClass "/Game/Breakout/Core/Actors/BP_Ball.BP_Ball_C" (Transformation|GetWorldTransform (Variables|Default|GetArrow)) "AlwaysSpawn" 0 0))
    (Variables|Default|SetBallRef _returnvalue)))

(event Custom|ResetPlayerPosition
  (bind _locationplayer (Variables|Default|GetLocationPlayer))
  ;[1 1 1] Reset la position du joueur
  (Transformation|SetActorLocation _locationplayer false false)
  (Transformation|SetWorldLocation (Variables|Default|GetSM_Paddle) _locationplayer false false))

(event EventBeginPlay
  ;[1 1 1] Obtenir le Mode de jeu du casse brique
  (bind _asbp_game_mode_breakout (Utilities|Casting|CastToBP_GameModeBreakout (Game|GetGameMode)))
  (Variables|Default|SetGameMode _asbp_game_mode_breakout)
  ;[1 1 1] Sauvegarde localisation du Start player
  (Variables|Default|SetLocationPlayer (Transformation|GetActorLocation))
  ;[1 1 1] Bind event
  (CallFunction|SpawnNewBall)
  (EventDispatchers|BindEventtoResetPositionPlayer (Variables|Default|GetGameMode) (delegate Custom|ResetPlayerPosition))
  (EventDispatchers|BindEventtoPlayGame (Variables|Default|GetGameMode) (delegate Custom|SpawnNewBall)))

(event Input|ActionEvents|InputActionShoot
  (params (Key :type Key%20Structure :default "None"))
  ;[1 1 1] Lancer la balle
  (:Pressed
    (bind _ballref (Variables|Default|GetBallRef)
      (:then
        (if (and (Utilities|IsValid _ballref) (not (Variables|/Game/Breakout/Core/Actors/BP_Ball.BP_Ball_C|GetbPlayerActive _ballref)))
          (Default|Lancer _ballref (Math|Rotator|GetRotationXVector (Transformation|GetWorldRotation (Variables|Default|GetArrow))))))
      (:else))))

(event Input|AxisEvents|InputAxisVerMove
  (params (AxisValue :type Float%20%28single-precision%29))
  ;[1 1 1] Deplacement
  ;;[1 1 1] Deplacement vertical
  (if (Variables|Default|GetbModeVerticalEnabled)
    (if (== (Variables|/Game/Breakout/Core/Engine/BP_GameModeBreakout.BP_GameModeBreakout_C|GetStatsGame (Variables|Default|GetGameMode)) 0)
      (Physics|AddImpulse (Variables|Default|GetSM_Paddle) (Math|Vector|MakeVector 0.0 (* AxisValue (Variables|Default|GetSpeed)) 0.0) "None" false))))

(event Input|AxisEvents|InputAxisHorMove
  (params (AxisValue :type Float%20%28single-precision%29))
  ;[1 1 1] Deplacement
  ;;[1 1 1] Deplacement horizontal
  (if (== (Variables|/Game/Breakout/Core/Engine/BP_GameModeBreakout.BP_GameModeBreakout_C|GetStatsGame (Variables|Default|GetGameMode)) 0)
    (Physics|AddImpulse (Variables|Default|GetSM_Paddle) (Math|Vector|MakeVector (* AxisValue (Variables|Default|GetSpeed)) 0.0 0.0) "None" false)))

(fn ConstructionScript)