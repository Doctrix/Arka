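; Breakout game mode that runs a brick-breaker round, tracking balls, score and collected gold and pushing them to the HUD widget.
; ResetLeJeu reloads the streamed level, resets counters and calls dispatchers to reset the player and start play.
; Lost balls cost a point; losing one with none left ends the game after a delay.
; The final score is inserted into the saved score list via DoOnce, saved and shown in a scoreboard widget.
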(event Custom|ResetLeJeu
  (bind _ballmax (Variables|Default|GetBallMax))
  (bind _gui_breakout (Variables|Default|GetGUI_Breakout))
  ;[1 1 1] reset le jeu
  (CallFunction|ChargerNiveau)
  (Variables|Default|SetBallActuel _ballmax)
  (Variables|/Game/Breakout/Core/Widgets/WBP_IU_Breakout.WBP_IU_Breakout_C|SetBillesDisponibles _gui_breakout _ballmax)
  (Variables|/Game/Breakout/Core/Widgets/WBP_IU_Breakout.WBP_IU_Breakout_C|SetScoreDuJoueur _gui_breakout 0)
  (Variables|/Game/Breakout/Core/Widgets/WBP_IU_Breakout.WBP_IU_Breakout_C|SetOrRecolter _gui_breakout 0)
  (Variables|Default|SetScoreActuel 0)
  (Default|CallResetPositionPlayer)
  (Variables|Default|SetStatsDuJeu "NewEnumerator0")
  (Default|CallPlayGame))

(event Custom|MajDuScore
  (params (Points :type Integer))
  (bind _gui_breakout (Variables|Default|GetGUI_Breakout))
  ;[1 1 1] Mise à jour du score
  (if (< (+ Points (Variables|Default|GetScoreActuel)) 0)
    (Variables|Default|SetScoreActuel 0)
    (else
      (Variables|Default|SetScoreActuel (+ Points (Variables|Default|GetScoreActuel)))))
  (bind _output_get (Variables|/Game/Breakout/Core/Widgets/WBP_IU_Breakout.WBP_IU_Breakout_C|SetScoreDuJoueur _gui_breakout (Variables|Default|GetScoreActuel)))
  (Variables|/Game/Breakout/Core/Widgets/WBP_ScreenEcranEndGame.WBP_ScreenEcranEndGame_C|SetScoreFinal (Variables|/Game/Breakout/Core/Widgets/WBP_IU_Breakout.WBP_IU_Breakout_C|GetEcranFinMiniJeu_WBP _gui_breakout) _output_get))

(event Custom|BallPerdu
  ;[1 1 1] Ball perdu ( 1 points de moins)
  (CallFunction|MajDuScore -1)
  (if (<= (Variables|Default|GetBallActuel) 0)
    (CallFunction|FinDePartie)
    (else
      (bind _output_get (Variables|Default|SetBallActuel (- (Variables|Default|GetBallActuel) 1)))
      (Variables|/Game/Breakout/Core/Widgets/WBP_IU_Breakout.WBP_IU_Breakout_C|SetBillesDisponibles (Variables|Default|GetGUI_Breakout) _output_get))))

(event Custom|FinDePartie
  ;[1 1 1] Fin de partie
  (Variables|Default|SetStatsDuJeu "NewEnumerator0")
  (Variables|Default|SetFinDePartie_CasseBrique true)
  (Utilities|FlowControl|Delay 2.0)
  (CallFunction|AfficherLeTableauDesScores))

(event Custom|ChargerNiveau
  (bind _returnvalue (Utilities|Name|MakeLiteralName "CB_Niveau001"))
  ;[1 1 1] Charger le niveau
  (Game|UnloadStreamLevel(byName) _returnvalue false)
  (Game|LoadStreamLevel(byName) _returnvalue true))

(event Custom|OrRecolterParLeJoueur
  (params (Or :type Integer))
  ;[1 1 1] Or recolter
  (Variables|Default|SetOrRecolterActuel (+ Or (Variables|Default|GetOrRecolterActuel)))
  (Variables|/Game/Breakout/Core/Widgets/WBP_IU_Breakout.WBP_IU_Breakout_C|SetOrRecolter (Variables|Default|GetGUI_Breakout) (Variables|Default|GetOrRecolterActuel)))

(event Custom|AfficherLeTableauDesScores
  (bind _scoreactuel (Variables|Default|GetScoreActuel))
  (bind _scoreofplayer (Variables|Default|GetScoreOfPlayer))
  ;[1 1 1] Afficher le tableau des score et sauvegarder
  (if (Variables|Default|GetFinDePartie_CasseBrique)
    (bind _returnvalue (SaveGame|LoadGamefromSlot (Variables|Default|GetSauvegardeScore_CB)))
    (bind _asbp_save_game (Utilities|Casting|CastToBP_SaveGame _returnvalue)
      (:then
        (for _array_element (Variables|/Game/Breakout/Core/BP_SaveGame.BP_SaveGame_C|GetScorePlayer _asbp_save_game)
          (Utilities|FlowControl|Sequence
            (:then_0
              (if (<= (.Score (Utilities|Struct|BreakS_ScorePlayer _array_element)) _scoreactuel)
                (Utilities|FlowControl|DoOnce false
                  (:Completed
                    (Utilities|Array|Add (Variables|Default|GetScoreOfPlayer) (Utilities|Struct|MakeS_ScorePlayer "None" _scoreactuel (Class|KismetMathLibrary|GetDate)))))))
            (:then_1
              (Utilities|Array|Add _scoreofplayer _array_element))))
        (Utilities|FlowControl|Sequence
          (:then_0
            (Utilities|FlowControl|DoOnce false :!label _label
              (:Completed
                (Utilities|Array|Add (Variables|Default|GetScoreOfPlayer) (Utilities|Struct|MakeS_ScorePlayer "None" _scoreactuel (Class|KismetMathLibrary|GetDate))))))
          (:then_1
            (bind _returnvalue_2 (SaveGame|CreateSaveGameObject "/Game/Breakout/Core/BP_SaveGame.BP_SaveGame_C" :!label _label_2))
            (Variables|/Game/Breakout/Core/BP_SaveGame.BP_SaveGame_C|SetScorePlayer (.AsBP%20Save%20Game (Utilities|Casting|CastToBP_SaveGame _returnvalue_2)) _scoreofplayer)
            (SaveGame|SaveGametoSlot _returnvalue_2 (Variables|Default|GetSauvegardeScore_CB))
            (Widget|RemovefromParent (Variables|Default|GetGUI_Breakout))
            (bind _returnvalue_3 (UserInterface|CreateWidget "/Game/Breakout/Core/Widgets/Scoreboard/TableauDesScores.TableauDesScores_C" 0 _scoreofplayer))
            (UserInterface|Viewport|AddtoViewport _returnvalue_3 0))))
      (:CastFailed
        (Utilities|FlowControl|Sequence
          (:then_0
            (goto _label))
          (:then_1
            (goto _label_2)))))))

(event EventBeginPlay
  (bind _returnvalue (UserInterface|CreateWidget "/Game/Breakout/Core/Widgets/WBP_IU_Breakout.WBP_IU_Breakout_C"))
  (bind _output_get (Variables|Default|SetGUI_Breakout _returnvalue))
  (UserInterface|Viewport|AddtoViewport _output_get 0)
  (CallFunction|ResetLeJeu))

(event EventTick
  (params (DeltaSeconds :type Float%20%28single-precision%29)))

(fn ConstructionScript)