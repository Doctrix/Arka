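; Breakout button that keeps mouse hover and keyboard focus in sync and restyles itself to show which is active.
; Start launches a looping timer that polls CheckFocus instead of relying on hover or focus events.
; When hovered, the button takes keyboard focus and uses the mouse style; otherwise it switches between selected and unselected styles based on whether it has focus.
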(fn Start
  (Utilities|Time|SetTimerbyFunctionName 0 "CheckFocus" 0.1 true))

(fn CheckFocus
  (if (Widget|IsHovered)
    (Widget|SetKeyboardFocus)
    (Class|Button|SetStyle (Variables|Default|GetMouseStyle))
    (else
      (Class|Button|SetStyle (select (Class|Widget|HasKeyboardFocus) (Variables|Default|GetCleSelectionner) (Variables|Default|GetCleNoSelectionner))))))